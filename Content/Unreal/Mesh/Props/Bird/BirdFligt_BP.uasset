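; Bird prop Blueprint that moves a bird along a spline path.
; On BeginPlay a timeline starts, and its alpha, scaled by spline length, gives the distance along the spline.
; Each update sets the BirdFlightMorph component's relative transform from the spline's local location and rotation, with a yaw offset to orient the bird.
; The construction script applies the PlayRate variable to the timeline to control flight speed.
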(event `self.ReceiveBeginPlay`
  (bind (_direction _animation_alpha) (`Timeline|Timeline_0` :!via `PlayFromStart`)
    (:`Update`
      (bind _returnvalue (* _animation_alpha (`SplineComponent.GetSplineLength` (`self.Spline`))))
      (`SceneComponent.K2_SetRelativeTransform` (`self.BirdFlightMorph`) (`KismetMathLibrary.MakeTransform` (`SplineComponent.GetLocationAtDistanceAlongSpline` (`self.Spline`) _returnvalue "Local") (`KismetMathLibrary.MakeRotator` (.roll (`SplineComponent.GetRotationAtDistanceAlongSpline` (`self.Spline`) _returnvalue "Local")) (.pitch (`SplineComponent.GetRotationAtDistanceAlongSpline` (`self.Spline`) _returnvalue "Local")) (+ (.yaw (`SplineComponent.GetRotationAtDistanceAlongSpline` (`self.Spline`) _returnvalue "Local")) 90.0)) (1.0 1.0 1.0)) false false))))

(fn `UserConstructionScript`
  (`TimelineComponent.SetPlayRate` (`self.Timeline_0`) (`self.PlayRate`)))