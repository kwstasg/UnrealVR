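; Elevator actor for the NyLeve level that travels while a Character stands in its trigger Box and returns after they leave.
; Construction script caches start and end world locations from two mesh components, and a timeline lerps the whole actor between them via relative location.
; Overlap plays the timeline forward; end overlap reverses it after a short delay.
; A door sound plays during travel, replaced by two stop sounds when the timeline finishes.
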(event `self.Box.OnComponentBeginOverlap`
  (params (OverlappedComponent :type "PrimitiveComponent Object Reference") (OtherActor :type "Actor Object Reference") (OtherComp :type "PrimitiveComponent Object Reference") (OtherBodyIndex :type Integer) (bFromSweep :type Boolean) (SweepResult :type "HitResult Structure (by ref)"))
  (cast `Character` OtherActor)
  (`AudioComponent.Play` (`self.DoorsMod_General_mdoorL20`) 0.0)
  (bind (_direction _duration) (`Timeline|Timeline_0` :!label _label)
    (:`Update`
      (`self.K2_SetActorRelativeLocation` (`KismetMathLibrary.VLerp` (`self.StartLocation`) (`self.EndLocation`) _duration)))
    (:`Finished`
      (`AudioComponent.Stop` (`self.DoorsMod_General_mdoorL20`))
      (`AudioComponent.Play` (`self.DoorsMod_General_mdend51`) 0.0)
      (`AudioComponent.Play` (`self.DoorsMod_General_mdoorS23`) 0.0))))

(event `self.Box.OnComponentEndOverlap`
  (params (OverlappedComponent :type "PrimitiveComponent Object Reference") (OtherActor :type "Actor Object Reference") (OtherComp :type "PrimitiveComponent Object Reference") (OtherBodyIndex :type Integer))
  (cast `Character` OtherActor)
  (`KismetSystemLibrary.Delay` 1.5)
  (`AudioComponent.Play` (`self.DoorsMod_General_mdoorL20`) 0.0)
  (goto _label :!via `Reverse`))

(fn `UserConstructionScript`
  (set `self.StartLocation` (`SceneComponent.K2_GetComponentLocation` (`self.StaticMeshComponent`)))
  (set `self.EndLocation` (`SceneComponent.K2_GetComponentLocation` (`self.StaticMeshEndLocation`))))