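; Overlap-triggered switch for an elevator in the NyLeve level, which calls its linked Elevator when a Character steps into its Box.
; A timeline, restarted only when not already playing, lerps the switch actor from start to end location, plays a click sound from an event track, then calls CallElevator when finished.
; The Construction Script derives both endpoints from the Switch component's world location and EndLocationOffset, though movement sets the actor's relative location.
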(event `self.Box.OnComponentBeginOverlap`
  (params (OverlappedComponent :type "PrimitiveComponent Object Reference") (OtherActor :type "Actor Object Reference") (OtherComp :type "PrimitiveComponent Object Reference") (OtherBodyIndex :type Integer) (bFromSweep :type Boolean) (SweepResult :type "HitResult Structure (by ref)"))
  (cast `Character` OtherActor)
  (if (not (`TimelineComponent.IsPlaying` (`self.Timeline_0`)))
    (bind (_direction _duration) (`Timeline|Timeline_0` :!via `PlayFromStart`)
      (:`Update`
        (`self.K2_SetActorRelativeLocation` (`KismetMathLibrary.VLerp` (`self.StartLocation`) (`self.EndLocation`) _duration)))
      (:`Finished`
        (`/Game/Unreal/Blueprints/NyLeve-U1/NyLeve-Elevator02_BP. CallElevator` (`self.Elevator`)))
      (:`Switch Play SFX`
        (`AudioComponent.Play` (`self.Activates_ClicksBig_start14`) 0.0)))))

(fn `UserConstructionScript`
  (set `self.StartLocation` (`SceneComponent.K2_GetComponentLocation` (`self.Switch`)))
  (set `self.EndLocation` (+ (`SceneComponent.K2_GetComponentLocation` (`self.Switch`)) (`self.EndLocationOffset`))))