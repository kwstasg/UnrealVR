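; Elevator Blueprint for the Vortex2-U1 map that moves a brush mover mesh along a spline.
; ElevatorDown plays a timeline from the start and ElevatorUp reverses it, with its alpha scaled by spline length to set the mesh's relative location, without rotation.
; Timeline SFX events check playback direction, so the moving sound and the stopping sounds swap correctly when reversed.
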(event `Elevator Down`
  (bind (_direction _animation_alpha) (`Timeline|Timeline_0` :!via `PlayFromStart` :!label _label)
    (:`Update`
      (`SceneComponent.K2_SetRelativeTransform` (`self.Mover49_Brush_StaticMesh`) (`KismetMathLibrary.MakeTransform` (`SplineComponent.GetLocationAtDistanceAlongSpline` (`self.Spline`) (* _animation_alpha (`SplineComponent.GetSplineLength` (`self.Spline`))) "Local")) false false))
    (:`Play SFX`
      (bind _returnvalue (`|EnumEquality` _direction "Forward"))
      (if _returnvalue
        (`AudioComponent.Play` (`self.DoorsMod_General_mdoorL20`) 0.0 :!label _label_2)
        (else
          (`AudioComponent.Stop` (`self.DoorsMod_General_mdoorL20`) :!label _label_3)
          (`AudioComponent.Play` (`self.DoorsMod_General_mdend51`) 0.0)
          (`AudioComponent.Play` (`self.DoorsMod_General_mdoorS23`) 0.0))))
    (:`Stop SFX`
      (if _returnvalue
        (goto _label_3)
        (else
          (goto _label_2))))))

(event `Elevator Up`
  (goto _label :!via `Reverse`))

(fn `UserConstructionScript`)