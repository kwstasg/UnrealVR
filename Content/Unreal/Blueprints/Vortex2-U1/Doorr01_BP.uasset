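; Automatic sliding door that opens when a Character enters its trigger box and closes after a short delay when one leaves.
; The construction script caches world locations of start and end marker components.
; A timeline lerps the start component between those locations, playing forward on overlap and reversing on exit.
; A door sound plays on both opening and closing.
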(event `self.Box.OnComponentBeginOverlap`
  (params (OverlappedComponent :type "PrimitiveComponent Object Reference") (OtherActor :type "Actor Object Reference") (OtherComp :type "PrimitiveComponent Object Reference") (OtherBodyIndex :type Integer) (bFromSweep :type Boolean) (SweepResult :type "HitResult Structure (by ref)"))
  (cast `Character` OtherActor)
  (`AudioComponent.Play` (`self.DoorsMod_General_mdoorE21`) 0.0)
  (bind (_direction _duration) (`Timeline|Timeline_0` :!label _label)
    (:`Update`
      (`SceneComponent.K2_SetWorldLocation` (`self.DoorStartLocation`) (`KismetMathLibrary.VLerp` (`self.StartLocation`) (`self.EndLocation`) _duration) false false))))

(event `self.Box.OnComponentEndOverlap`
  (params (OverlappedComponent :type "PrimitiveComponent Object Reference") (OtherActor :type "Actor Object Reference") (OtherComp :type "PrimitiveComponent Object Reference") (OtherBodyIndex :type Integer))
  (cast `Character` OtherActor)
  (`KismetSystemLibrary.Delay` 0.5)
  (`AudioComponent.Play` (`self.DoorsMod_General_mdoorE21`) 0.0)
  (goto _label :!via `Reverse`))

(fn `UserConstructionScript`
  (set `self.StartLocation` (`SceneComponent.K2_GetComponentLocation` (`self.DoorStartLocation`)))
  (set `self.EndLocation` (`SceneComponent.K2_GetComponentLocation` (`self.DoorEndLocation`))))