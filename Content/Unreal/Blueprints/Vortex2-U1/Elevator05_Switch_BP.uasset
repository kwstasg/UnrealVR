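; Elevator switch actor that animates and drives a referenced elevator when a Character overlaps its box.
; The construction script derives start and end location and rotation from the Switch component's world transform.
; On overlap, unless already playing, a timeline lerps the actor's relative transform between them.
; Timeline event tracks play the click sound and call ElevatorUp and ElevatorDown on the elevator.
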(event `self.Box.OnComponentBeginOverlap`
  (params (OverlappedComponent :type "PrimitiveComponent Object Reference") (OtherActor :type "Actor Object Reference") (OtherComp :type "PrimitiveComponent Object Reference") (OtherBodyIndex :type Integer) (bFromSweep :type Boolean) (SweepResult :type "HitResult Structure (by ref)"))
  (cast `Character` OtherActor)
  (if (not (`TimelineComponent.IsPlaying` (`self.Timeline_0`)))
    (bind (_direction _rotation_alpha _location_alpha) (`Timeline|Timeline_0` :!via `PlayFromStart`)
      (:`Update`
        (`self.K2_SetActorRelativeRotation` (`KismetMathLibrary.RLerp` (`self.StartRotation`) (`self.EndRotation`) _rotation_alpha))
        (`self.K2_SetActorRelativeLocation` (`KismetMathLibrary.VLerp` (`self.StartLocation`) (`self.EndLocation`) _location_alpha)))
      (:`Switch Play SFX`
        (`AudioComponent.Play` (`self.Activates_ClicksBig_start14`) 0.0))
      (:`GoUp`
        (`/Game/Unreal/Blueprints/Vortex2-U1/Elevator05_BP.Elevator Up` (`self.Elevator`)))
      (:`GoDown`
        (`/Game/Unreal/Blueprints/Vortex2-U1/Elevator05_BP.Elevator Down` (`self.Elevator`))))))

(fn `UserConstructionScript`
  (bind (_returnvalue_roll _returnvalue_pitch _returnvalue_yaw) (`KismetMathLibrary.BreakRotator` (`SceneComponent.K2_GetComponentRotation` (`self.Switch`))))
  (set `self.StartLocation` (`SceneComponent.K2_GetComponentLocation` (`self.Switch`)))
  (set `self.StartRotation` (`SceneComponent.K2_GetComponentRotation` (`self.Switch`)))
  (set `self.EndLocation` (+ (`SceneComponent.K2_GetComponentLocation` (`self.Switch`)) (0.0 -60.0 0.0)))
  (set `self.EndRotation` (`KismetMathLibrary.MakeRotator` _returnvalue_roll (+ _returnvalue_pitch -270.0) _returnvalue_yaw)))