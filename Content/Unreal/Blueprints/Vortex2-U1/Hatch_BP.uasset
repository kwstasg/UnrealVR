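; Hatch actor that swings open on demand and serves as a level transition to NyLeve-U1.
; OpenHatch plays a door motor sound while a timeline rotates HatchPivot open, then stops it and plays a click when finished.
; A Box trigger opens the NyLeve-U1 level when any Character overlaps it, independently of the hatch's open state.
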(event `Open Hatch`
  (`AudioComponent.Play` (`self.DoorsMod_General_mdoorL20`) 0.0)
  (bind (_direction _open_alpha) (`Timeline|Timeline_0`)
    (:`Update`
      (`SceneComponent.K2_SetRelativeRotation` (`self.Hatch Pivot`) (`KismetMathLibrary.RLerp` (struct) (struct :`Pitch` -110.0) _open_alpha) false false))
    (:`Finished`
      (`AudioComponent.Stop` (`self.DoorsMod_General_mdoorL20`))
      (`AudioComponent.Play` (`self.Activates_ClicksBig_start14`) 0.0))))

(event `self.Box.OnComponentBeginOverlap`
  (params (OverlappedComponent :type "PrimitiveComponent Object Reference") (OtherActor :type "Actor Object Reference") (OtherComp :type "PrimitiveComponent Object Reference") (OtherBodyIndex :type Integer) (bFromSweep :type Boolean) (SweepResult :type "HitResult Structure (by ref)"))
  (cast `Character` OtherActor)
  (`GameplayStatics.OpenLevel` "NyLeve-U1"))

(fn `UserConstructionScript`)